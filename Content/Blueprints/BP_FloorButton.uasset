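; BP_FloorButton is a floor button that switches every BP_MovingPlatform in the level between solid and non-colliding when something overlaps its trigger area.
; Each begin overlap, with no filter on the overlapping actor, gathers all platforms and uses PlatformToggle to choose whether to enable or disable their collision.
; Both branches flip platform visibility and invert PlatformToggle inside the loop; the disabling branch also prints a debug message.
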(event OnComponentBeginOverlap(ButtonTriggerArea)
  (params (OverlappedComponent :type Primitive%20Component%20Object%20Reference) (OtherActor :type Actor%20Object%20Reference) (OtherComp :type Primitive%20Component%20Object%20Reference) (OtherBodyIndex :type Integer) (bFromSweep :type Boolean) (SweepResult :type Hit%20Result%20Structure%20%28by%20ref%29))
  (bind _outactors (Actor|GetAllActorsOfClass "/Game/Blueprints/BP_MovingPlatform.BP_MovingPlatform_C"))
  (if (== (Variables|Default|GetPlatformToggle) true)
    (for _array_element _outactors
      (Collision|SetCollisionEnabled (Variables|/Game/Blueprints/BP_MovingPlatform.BP_MovingPlatform_C|GetPlatform _array_element) "QueryAndPhysics")
      (Rendering|ToggleVisibility (Variables|/Game/Blueprints/BP_MovingPlatform.BP_MovingPlatform_C|GetPlatform _array_element) false)
      (Variables|Default|SetPlatformToggle false))
    (else
      (for _array_element_2 _outactors
        (Collision|SetCollisionEnabled (Variables|/Game/Blueprints/BP_MovingPlatform.BP_MovingPlatform_C|GetPlatform _array_element_2) "NoCollision")
        (Rendering|ToggleVisibility (Variables|/Game/Blueprints/BP_MovingPlatform.BP_MovingPlatform_C|GetPlatform _array_element_2) false)
        (Variables|Default|SetPlatformToggle true))
      (Development|PrintString "DONE"))))

(fn ConstructionScript)